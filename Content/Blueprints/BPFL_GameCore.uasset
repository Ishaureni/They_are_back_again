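; Blueprint function library that supplies shared tile grid math for converting tile coordinates to world positions.
; GetTileWorldPosition scales the X and Y tile coordinates by tile size plus padding and takes Z from a given height.
; Size and padding come from constant getter functions, with padding currently zero, so the grid is anchored at the world origin with tiles spaced by their size alone.
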(fn `GetMyTileSize`
  (returns (result :type "Float (double-precision)"))
  (return 100.0))

(fn `GetTilePadding`
  (returns (Padding :type "Float (double-precision)"))
  (return 0.0))

(fn `GetTileWorldPosition`
  (params (TileCoord :type "/Game/Blueprints/Sturctures/IntVector2D Structure") (Height :type "Float (double-precision)"))
  (returns (NewParam :type "Vector Structure"))
  (bind (_x _y) (break `/Game/Blueprints/Sturctures/IntVector2D` TileCoord))
  (bind _returnvalue (+ (`self.GetMyTileSize` null) (`self.GetTilePadding` null)))
  (return (`KismetMathLibrary.MakeVector` (* _x _returnvalue) (* _y _returnvalue) Height)))